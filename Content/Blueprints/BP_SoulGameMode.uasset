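; BP_SoulGameMode is a game mode Blueprint that holds a current game state and drives the HUD from it.
; On BeginPlay it casts the first player controller's HUD to BP_HUD and stores it.
; ChangeState switches on the requested state and tells the HUD to show its main menu state, the only case wired.
; Tick switches on CurrentState but runs no logic yet.
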(event `self.ReceiveBeginPlay`
  (bind _asbp_hud (cast `/Game/UI/BP_HUD` (`PlayerController.GetHUD` (`GameplayStatics.GetPlayerController` 0))))
  (set `self.OurHud` _asbp_hud))

(event `self.ReceiveTick`
  (params (DeltaSeconds :type "Float (single-precision)"))
  (switch `/Game/Blueprints/E_GameState` (`self.CurrentState`)))

(fn `ChangeState`
  (params (InState :type "/Game/Blueprints/E_GameState Enum" :default "NewEnumerator0"))
  (switch `/Game/Blueprints/E_GameState` InState
    (:`NewEnumerator0`
      (`/Game/UI/BP_HUD.MainMenuState` (`self.OurHud`)))))

(fn `UserConstructionScript`)