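; Game mode that links level and game state held in BP_SoulsGameInstance to the state screens of BP_HUD_LevelAndState.
; On BeginPlay it shows the loading, main menu or in-game HUD state, then registers itself with the game instance via FinishGameModeLoad.
; State changes are forwarded to the game instance with or without loading.
; It also relays end-of-loading and death to the HUD, checks level load completion, and quits after a short delay.
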(event `self.ReceiveBeginPlay`
  (bind _asbp_hud_level_and_state (cast `/Game/UI/BP_HUD_LevelAndState` (`PlayerController.GetHUD` (`GameplayStatics.GetPlayerController` 0))))
  (bind _output_get (set `self.OurHud` _asbp_hud_level_and_state))
  (bind _asbp_souls_game_instance (cast `/Game/Blueprints/BP_SoulsGameInstance` (`GameplayStatics.GetGameInstance`)))
  (if (`/Game/Blueprints/BP_SoulsGameInstance.Need Loading` _asbp_souls_game_instance)
    (`/Game/UI/BP_HUD_LevelAndState.Loading State` _output_get)
    (else
      (switch `/Game/Blueprints/E_GameState` (`/Game/Blueprints/BP_SoulsGameInstance.CurrentGameState` _asbp_souls_game_instance)
        (:`NewEnumerator0`
          (`/Game/UI/BP_HUD_LevelAndState.Main Menu State` _output_get))
        (:`NewEnumerator2`
          (`/Game/UI/BP_HUD_LevelAndState.In Game State` _output_get)))))
  (`/Game/Blueprints/BP_SoulsGameInstance.FinishGameModeLoad` _asbp_souls_game_instance self))

(event `Game End`
  (`KismetSystemLibrary.Delay` 0.5)
  (`KismetSystemLibrary.QuitGame` null "Quit"))

(fn `ChangeState`
  (params (InState :type "/Game/Blueprints/E_GameState Enum" :default "NewEnumerator0"))
  (bind _asbp_souls_game_instance (cast `/Game/Blueprints/BP_SoulsGameInstance` (`GameplayStatics.GetGameInstance`)))
  (`/Game/Blueprints/BP_SoulsGameInstance.ChangeState` _asbp_souls_game_instance InState false)
  (`KismetSystemLibrary.PrintString` "Hello"))

(fn `ChangeStateWithLoading`
  (params (InputPin :type "/Game/Blueprints/E_GameState Enum" :default "NewEnumerator2"))
  (bind _asbp_souls_game_instance (cast `/Game/Blueprints/BP_SoulsGameInstance` (`GameplayStatics.GetGameInstance`)))
  (`/Game/Blueprints/BP_SoulsGameInstance.ChangeState` _asbp_souls_game_instance (`local.InputPin`) true))

(fn `CheckLevelLoadFinished`
  (returns (ReturnValue :type Boolean))
  (bind _returnvalue (`self.GetLevel`))
  (`/Engine/EditorBlueprintResources/StandardMacros.IsValid` _returnvalue
    (:`Is Valid`
      (bind _returnvalue_2 (message `AssetRegistry.IsSearchAllAssets` _returnvalue))
      (return _returnvalue_2))))

(fn `EndLoading`
  (`/Game/UI/BP_HUD_LevelAndState.End Loading` (`self.OurHud`)))

(fn `UserConstructionScript`)

(fn `YouDie`
  (bind _ourhud (`self.OurHud`))
  (`/Game/UI/BP_HUD_LevelAndState.Transition Phase` _ourhud)
  (`/Game/UI/BP_HUD_LevelAndState.You Die State` _ourhud))