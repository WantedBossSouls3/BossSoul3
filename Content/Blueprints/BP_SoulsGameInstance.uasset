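; Game instance for a souls-like game that tracks the game state and drives level changes.
; ChangeState opens the main menu or demo map, or tells the current game mode to run its death handling.
; Level changes clear a game-mode loading flag, which FinishGameModeLoad sets again while storing the new game mode.
; It also applies brightness through a tonemapper gamma console command.
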(fn `Apply Brightness`
  (`KismetSystemLibrary.ExecuteConsoleCommand` (`KismetStringLibrary.Concat_StrStr` "r.TonemapperGamma " (`KismetStringLibrary.Conv_DoubleToString` (`self.Brightness`))) null))

(fn `ChangeLevel`
  (params (`Open Level` :type "World Soft Object Reference" :default "/Game/Maps/EntryLevel.EntryLevel"))
  (set `self.GameMode Loading` false)
  (`GameplayStatics.OpenLevelBySoftObjectPtr` `Open Level`))

(fn `ChangeState`
  (params (InState :type "/Game/Blueprints/E_GameState Enum" :default "NewEnumerator0") (bNeedLoading :type Boolean))
  (locals (PrevState :type "/Game/Blueprints/E_GameState Enum"))
  (set `local.PrevState` (`self.CurrentGameState`))
  (`|ExecutionSequence`
    (:`then_0`
      (bind _output_get (set `self.CurrentGameState` (`local.InState`)))
      (switch `/Game/Blueprints/E_GameState` _output_get
        (:`NewEnumerator0`
          (`self.ChangeLevel` "/Game/Maps/MainMenuLevel.MainMenuLevel"))
        (:`NewEnumerator2`
          (`self.ChangeLevel` "/Game/EnvironmentPack2/Maps/DemoMap1.DemoMap1"))
        (:`NewEnumerator3`
          (`/Game/Blueprints/BP_SoulGameMode_LevelAndState.YouDie` (`self.CurrentGameMode`)))))
    (:`then_1`
      (set `self.Need Loading` (`local.bNeedLoading`)))))

(fn `FinishGameModeLoad`
  (params (UpdatedGameMode :type "/Game/Blueprints/BP_SoulGameMode_LevelAndState Object Reference"))
  (set `self.CurrentGameMode` UpdatedGameMode)
  (set `self.GameMode Loading` true))