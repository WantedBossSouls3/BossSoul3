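; BP_Boss is a boss character that rotates toward, chases and combo-attacks the player while able to act.
; It wires action, weapon and status components together on BeginPlay, then deactivates until an activate event, with level reset deactivating it again.
; Tick gates movement and attacks on groggy, death and player critical-attack state.
; Overlap volumes handle kick damage and the groggy critical-hit window, with helpers for parry and critical-hit reactions.
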(event `self.ReceiveBeginPlay`
  (`self.SetAboutActionComp`)
  (`self.SetAboutWeaponComp`)
  (`self.SetAboutStatusComp`)
  (`self.SetAboutPlayer`)
  (bind _asbp_soul_game_mode_level_and_state (cast `/Game/Blueprints/BP_SoulGameMode_LevelAndState` (`GameplayStatics.GetGameMode`)))
  (add `/Game/Blueprints/BP_SoulGameMode_LevelAndState.ResetBossLevel` _asbp_soul_game_mode_level_and_state (delegate `/Game/Utility/BPI_OnOff.Deactivate`))
  (add `self.BossActivate` (delegate `/Game/Utility/BPI_OnOff.Activate`))
  (`PrimitiveComponent.SetCollisionEnabled` (`self.KickCapsule`) "NoCollision")
  (`PrimitiveComponent.SetCollisionEnabled` (`self.CriticalEnableBox`) "NoCollision")
  (`self.Deactivate`))

(event `/Game/Utility/BPI_OnOff.Activate`
  (`/Game/Boss/Character/Status/StatusComp.InitStatus` (`self.StatusComp`))
  (`/Game/Boss/Character/Action/ActionComp.InitActions` (`self.BossActionComp`))
  (`self.SetAboutPlayer`))

(event `/Game/Utility/BPI_OnOff.Deactivate`
  (`/Game/Boss/Character/Action/ActionComp.Do Action Something` (`self.BossActionComp`)))

(event `self.ReceiveTick`
  (params (DeltaSeconds :type "Float (single-precision)"))
  (bind _bossactioncomp (`self.BossActionComp`))
  (bind _targetplayer (`self.TargetPlayer`))
  (if (`self.CheckCondition`)
    (if (!= (`/Game/Player/BP_PlayerCharacter.CriticalAttackState` (`self.TargetPlayer`)) 1)
      (if (`self.InBoundary` (`self.AttackBoundary`))
        (`/Game/Boss/Character/Action/ActionComp.ComboAttack` (`self.BossActionComp`)))
      (if (`/Game/Boss/Character/Action/ActionComp.CanMove` (`self.BossActionComp`))
        (`|ExecutionSequence`
          (:`then_0`
            (`/Engine/EditorBlueprintResources/StandardMacros.IsValid` _targetplayer
              (:`Is Valid`
                (`/Game/Boss/Character/Action/ActionComp.Rotate` _bossactioncomp (`/Game/Boss/Character/Action/ActionComp.CalcRotationToDest` _bossactioncomp (`self.K2_GetActorLocation` _targetplayer)) DeltaSeconds))))
          (:`then_1`
            (set `self.bDeccel` (`self.InBoundary` (`self.MoveBoundary`)))
            (`self.MoveMacro` DeltaSeconds))))
      (else
        (`self.PlayAnimMontage` "/Game/Boss/Character/Animation/Critical_get_hit_02_Montage.Critical_get_hit_02_Montage")))))

(event `self.KickCapsule.OnComponentBeginOverlap`
  (params (OverlappedComponent :type "PrimitiveComponent Object Reference") (OtherActor :type "Actor Object Reference") (OtherComp :type "PrimitiveComponent Object Reference") (OtherBodyIndex :type Integer) (bFromSweep :type Boolean) (SweepResult :type "HitResult Structure (by ref)"))
  (bind _asbp_player_character (cast `/Game/Player/BP_PlayerCharacter` OtherActor))
  (`/Game/Player/BP_PlayerCharacter.PlayerDamaged` _asbp_player_character (`self.Deal`)))

(event `self.CriticalEnableBox.OnComponentBeginOverlap`
  (params (OverlappedComponent :type "PrimitiveComponent Object Reference") (OtherActor :type "Actor Object Reference") (OtherComp :type "PrimitiveComponent Object Reference") (OtherBodyIndex :type Integer) (bFromSweep :type Boolean) (SweepResult :type "HitResult Structure (by ref)"))
  ; Groggy
  (if (`/Game/Boss/Character/Status/StatusComp.IsGroggyed` (`self.StatusComp`))
    (cast `/Game/Player/BP_PlayerCharacter` OtherActor)
    (set `/Game/Boss/Character/Status/StatusComp.CanBeCritacalAttacked` true (`self.StatusComp`))))

(event `self.CriticalEnableBox.OnComponentEndOverlap`
  (params (OverlappedComponent :type "PrimitiveComponent Object Reference") (OtherActor :type "Actor Object Reference") (OtherComp :type "PrimitiveComponent Object Reference") (OtherBodyIndex :type Integer))
  ; Groggy
  (if (`/Game/Boss/Character/Status/StatusComp.IsGroggyed` (`self.StatusComp`))
    (cast `/Game/Player/BP_PlayerCharacter` OtherActor)
    (set `/Game/Boss/Character/Status/StatusComp.CanBeCritacalAttacked` false (`self.StatusComp`))))

(fn `ChangeParryedStatus`
  (params (`CanBeParryed?` :type Boolean))
  (set `/Game/Boss/Character/Action/BossActionComp.CanBeParryed` `CanBeParryed?` (`self.BossActionComp`)))

(fn `CheckCondition`
  (returns (ReturnValue :type Boolean))
  (bind _statuscomp (`self.StatusComp`))
  (`/Engine/EditorBlueprintResources/StandardMacros.IsValid` (`self.TargetPlayer`)
    (:`Is Valid`
      (return (and (not (`/Game/Boss/Character/Status/StatusComp.IsGroggyed` _statuscomp)) (not (`/Game/Boss/Character/Status/StatusComp.IsDead` _statuscomp)) (`/Game/Boss/Character/Action/ActionComp.CanAct` (`self.BossActionComp`)))))
    (:`Is Not Valid`
      (`self.SetAboutPlayer`))))

(fn `EnemyDamaged`
  (params (Deal :type "Float (double-precision)"))
  (`/Game/Boss/Character/Status/StatusComp.Change HP` (`self.StatusComp`) Deal))

(fn `InBoundary`
  (params (B :type "Float (double-precision)"))
  (returns (`InBoundary?` :type Boolean))
  (return (> B (`/Game/Boss/Character/Action/ActionComp.CalcDistanceToDestInXY` (`self.BossActionComp`) (`self.ToTargetLocation`)))))

(fn `PullTargetFrontOfBoss`
  (returns (Location :type "Vector Structure") (Rotator :type "Rotator Structure"))
  (bind _returnvalue (`self.GetActorForwardVector`))
  (return (+ (`self.K2_GetActorLocation`) (* _returnvalue (`self.CriticalDist`))) (`KismetMathLibrary.MakeRotFromZX` (`self.GetActorUpVector` (`self.TargetPlayer`)) (* _returnvalue -1.0))))

(fn `ReceiveGroggyState`
  (params (State :type Integer))
  (switch `int` State
    (:`1`
      (`self.PlayAnimMontage` "/Game/Boss/Character/Animation/Critical_get_hit_02_Montage.Critical_get_hit_02_Montage")
      (set `/Game/Boss/Character/Status/StatusComp.CanBeCritacalAttacked` false (`self.StatusComp`)))
    (:`2`
      (`self.PlayAnimMontage` "/Game/Boss/Character/Animation/CriticalEnd_Montage.CriticalEnd_Montage"))))

(fn `SendGroggyState`
  (returns (IsGroggyed :type Boolean))
  (return (`/Game/Boss/Character/Status/StatusComp.CanBeCritacalAttacked` (`self.StatusComp`))))

(fn `SendHP`
  (returns (HP :type "/Game/Utility/F_ConsumableValue Structure"))
  (bind _value (`BlueprintMapLibrary.Map_Find` (`/Game/Boss/Character/Status/BPDA_Status.StatusMap` (`/Game/Boss/Character/Status/StatusComp.StatusData` (`self.StatusComp`))) "NewEnumerator0"))
  (return (make `/Game/Utility/F_ConsumableValue` (break `/Game/Boss/Character/Status/FStatusValue` _value) (`.Max_4_7BAE4A2045D9636CDA2F4996046231BE` (break `/Game/Boss/Character/Status/FStatusValue` _value)))))

(fn `SetAboutActionComp`
  (`/Game/Boss/Character/Action/ActionComp.ResetActions` (`self.BossActionComp`)))

(fn `SetAboutPlayer`
  (bind _asbp_player_character (cast `/Game/Player/BP_PlayerCharacter` (`GameplayStatics.GetPlayerPawn` 0)))
  (bind _output_get (set `self.TargetPlayer` _asbp_player_character))
  (set `/Game/Player/BP_PlayerCharacter.BossActor` self _output_get))

(fn `SetAboutStatusComp`
  (bind _output_get (set `/Game/Boss/Character/Action/BossActionComp.StatusComp` (`self.StatusComp`) (`self.BossActionComp`)))
  (set `/Game/Boss/Character/Status/StatusComp.StatusData` "/Game/Boss/Character/Status/DA_BossStatus.DA_BossStatus" _output_get)
  (set `/Game/Boss/Character/Status/StatusComp.IsDead` false _output_get))

(fn `SetAboutWeaponComp`
  (bind _bossactioncomp (`self.BossActionComp`))
  (bind _weaponcomp (`self.WeaponComp`))
  (`|ExecutionSequence`
    (:`then_0`
      (bind _derivedweapon (`/Game/Boss/Character/Weapon/WeaponComp.SpawnWeapon` _weaponcomp))
      (`/Game/Boss/Character/Weapon/WeaponComp.AttachWeapon` _weaponcomp)
      (bind _asbp_boss_weapon (cast `/Game/Boss/Character/Weapon/BP_BossWeapon` _derivedweapon))
      (set `/Game/Boss/Character/Weapon/BP_BossWeapon.Boss` self _asbp_boss_weapon)
      (set `/Game/Boss/Character/Action/BossActionComp.Derived Weapon` _asbp_boss_weapon _bossactioncomp)
      (set `/Game/Boss/Character/Action/ActionComp.ComboOrder` (make `/Game/Boss/Character/Action/ComboOrder` 0 (`BlueprintMapLibrary.Map_Length` (`/Game/Boss/Character/Weapon/Dats/BPDA_DefaultWeaponAction.ComboAttack` (`/Game/Boss/Character/Weapon/BP_BaseWeapon.WeaponData` _derivedweapon)))) _bossactioncomp))))

(fn `UserConstructionScript`)