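; BP_LockOnPoint is a world marker that shows the player's lock-on target on the boss.
; It finds the single BP_Boss at BeginPlay and polls the player character's LockedOn flag every Tick.
; While locked on, it reveals its mesh and then follows the boss's spine_03 socket; otherwise it hides the mesh.
; Paired visible and invisible flags keep visibility from being set again every frame.
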(event `self.ReceiveBeginPlay`
  (bind _returnvalue (`GameplayStatics.GetActorOfClass` "/Game/Boss/Character/BP_Boss.BP_Boss_C"))
  (set `self.BossActor` _returnvalue))

(event `self.ReceiveTick`
  (params (DeltaSeconds :type "Float (single-precision)"))
  (bind _asbp_player_character (cast `/Game/Player/BP_PlayerCharacter` (`GameplayStatics.GetPlayerPawn` 0)))
  (if (`/Game/Player/BP_PlayerCharacter.LockedOn?` _asbp_player_character)
    (if (`self.LockOnVisible`)
      (`self.K2_SetActorLocation` (`SceneComponent.GetSocketLocation` (`Character.Mesh` (`self.BossActor`)) "spine_03"))
      (else
        (`SceneComponent.SetVisibility` (`self.LockOnMesh`) true false)
        (set `self.LockOnVisible` true)
        (set `self.LockOnInvisible` false)))
    (elif (not (`self.LockOnInvisible`))
      (`SceneComponent.SetVisibility` (`self.LockOnMesh`) false false)
      (set `self.LockOnVisible` false)
      (set `self.LockOnInvisible` true))))

(fn `UserConstructionScript`)