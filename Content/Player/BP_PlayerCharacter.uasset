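; Player character for a souls-like boss fight, with a socketed weapon, combo and critical attacks, parry, block, roll, backstep and run.
; Tick plays death at zero HP, moves backsteps and turns body and camera toward the boss while locked on.
; One button rolls, runs or backsteps depending on movement and hold time.
; Montages drive actions, gated by CanAct and ComboState; PlayerDamaged skips damage when invincible and halves it when blocking.
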(event `self.ReceiveBeginPlay`
  ; Attach Weapon
  (bind _returnvalue (`|SpawnActorFromClass` "/Game/Player/BP_Weapon.BP_Weapon_C" (`SceneComponent.GetSocketTransform` (`self.Mesh`) "weapon_handgrip_r" "RTS_World") "Undefined" "MultiplyWithRoot" null null))
  (`self.K2_AttachToComponent` _returnvalue (`self.Mesh`) "weapon_handgrip_r" "SnapToTarget" "SnapToTarget" "SnapToTarget" true))

(event `InputAction|LockOn`
  (params (Key :type "Key Structure"))
  ; Lock On/Off
  (:`Pressed`
    (if (`self.LockedOn?`)
      (set `self.LockedOn?` false)
      (else
        (set `self.LockedOn?` true)))))

(event `self.ReceiveTick`
  (params (DeltaSeconds :type "Float (single-precision)"))
  (bind _bossactor (`self.BossActor`))
  (bind _capsulecomponent (`self.CapsuleComponent`))
  (bind _capsulecomponent_2 (`self.CapsuleComponent`))
  (bind _returnvalue (`KismetMathLibrary.MakeRotFromX` (- (`KismetMathLibrary.MakeVector` (.x (`SceneComponent.K2_GetComponentLocation` (`Actor.RootComponent` _bossactor))) (.y (`SceneComponent.K2_GetComponentLocation` (`Actor.RootComponent` _bossactor)))) (`SceneComponent.K2_GetComponentLocation` _capsulecomponent_2))))
  (if (<= (`self.PlayerHP`) 0.0)
    (`|PlayMontage` (`self.Mesh`) "/Game/Player/Animations/PlayerDead_AnimMontage.PlayerDead_AnimMontage")
    (else
      (if (`self.LockedOn?`)
        ; Locked On
        (`/Engine/EditorBlueprintResources/StandardMacros.IsValid` _bossactor
          (:`Is Valid`
            (set `self.CameraBasedMovementRotation` _returnvalue)
            (if (`self.Blocking?`)
              (`SceneComponent.K2_SetWorldRotation` _capsulecomponent_2 _returnvalue false false :!label _label)
              (elif (`self.Rolling?`)
                _
                (elif (`self.RollPressed?`)
                  _
                  (else
                    (goto _label)))))
            (`Controller.SetControlRotation` (`self.GetController`) _returnvalue))))
      (if (`self.Backstepping?`)
        ; Backstep (Moving Location)
        (set `self.CanAct?` false)
        (if (`self.LockedOn?`)
          (`SceneComponent.K2_SetWorldRotation` (`self.CapsuleComponent`) _returnvalue false false))
        (`SceneComponent.K2_SetWorldLocation` _capsulecomponent (+ (`SceneComponent.K2_GetComponentLocation` _capsulecomponent) (* (`SceneComponent.GetForwardVector` (`self.ArrowComp`)) (-9.0 -9.0 -9.0))) true false))
      ; Run/Roll/Backstep
      ;; Run
      (if (`self.RollPressed?`)
        (set `self.PressedTime` (+ (`GameplayStatics.GetWorldDeltaSeconds`) (`self.PressedTime`)))
        (if (> (`self.PressedTime`) 0.49)
          (set `CharacterMovementComponent.MaxWalkSpeed` 900.0 (`self.CharacterMovement`)))))))

(event `InputAction|Dodge/Run/Jump/Backstep`
  (params (Key :type "Key Structure"))
  (bind _charactermovement (`self.CharacterMovement`))
  (bind _charactermaxspeed (`self.CharacterMaxSpeed`))
  ; Run/Roll/Backstep
  (:`Pressed`
    ;; Roll
    (set `self.RollPressed?` true)
    (set `CharacterMovementComponent.MaxWalkSpeed` (`self.CharacterMaxSpeed`) (`self.CharacterMovement`)))
  (:`Released`
    ;; Backstep Animation
    (if (`self.Moving?`)
      (if (<= (`self.PressedTime`) 0.2)
        (set `self.RollPressed?` false)
        (set `self.Rolling?` true)
        (set `self.PressedTime` 0.0)
        (set `CharacterMovementComponent.MaxWalkSpeed` _charactermaxspeed _charactermovement)
        (if (`self.CanAct?`)
          (if (`self.LockedOn?`)
            (`self.K2_SetActorRotation` (`self.InputBasedMovementRotation`))
            (else
              (`self.K2_SetActorRotation` (`self.CameraBasedMovementRotation`))))
          (`|PlayMontage` (`self.Mesh`) "/Game/Player/Animations/Roll_AnimMontage.Roll_AnimMontage"
            (:`then`
              (`KismetSystemLibrary.Delay` 33.0)
              (set `self.Rolling?` false))))
        (else
          (set `self.RollPressed?` false)
          (set `self.PressedTime` 0.0)
          (set `CharacterMovementComponent.MaxWalkSpeed` _charactermaxspeed _charactermovement)))
      (elif (`self.CanAct?`)
        (set `self.Backstepping?` true)
        (`|PlayMontage` (`self.Mesh`) "/Game/Player/Animations/Backstep_AnimMontage.Backstep_AnimMontage"
          (:`then`
            (`KismetSystemLibrary.Delay` 0.6)
            (set `self.Backstepping?` false)
            (set `self.CanAct?` true)))))))

(event `InputAxis|MoveForward/Backward`
  (params (AxisValue :type "Float (single-precision)"))
  (bind _yaw (.yaw (`self.GetControlRotation`)))
  ; Character Movement
  (set `self.Moving?` true)
  (bind _returnvalue (`KismetMathLibrary.MakeVector` AxisValue (stale `InputAxis|MoveRight/Left` AxisValue)))
  (if (== _returnvalue (0.0 0.0 0.0))
    (set `self.Moving?` false))
  (if (`self.LockedOn?`)
    (bind _returnvalue_2 (`KismetMathLibrary.MakeRotator` 0.0 0.0 (+ (.yaw (`KismetMathLibrary.MakeRotFromX` _returnvalue)) _yaw)))
    (set `self.InputBasedMovementRotation` _returnvalue_2)
    (else
      (set `self.CameraBasedMovementRotation` _returnvalue_2)))
  (if (`self.CanAct?`)
    (`self.AddMovementInput` (`KismetMathLibrary.GetForwardVector` (`KismetMathLibrary.MakeRotator` 0.0 0.0 _yaw)) AxisValue)))

(event `InputAction|Attack(Righthand)`
  (params (Key :type "Key Structure"))
  (bind _bossactor (`self.BossActor`))
  ; Light Attack (Right Hand)
  (:`Pressed`
    (if (== (`self.ComboState`) 1)
      (`self.K2_SetActorRotation` (`self.CameraBasedMovementRotation`))
      (`|PlayMontage` (`self.Mesh`) "/Game/Player/Animations/LightAttack1_AnimMontage.LightAttack1_AnimMontage")
      (elif (== (`self.ComboState`) 2)
        (`self.K2_SetActorRotation` (`self.CameraBasedMovementRotation`))
        (`|PlayMontage` (`self.Mesh`) "/Game/Player/Animations/LightAttack2_AnimMontage.LightAttack2_AnimMontage")
        (elif (`self.CanAct?`)
          (`/Engine/EditorBlueprintResources/StandardMacros.IsValid` _bossactor
            (:`Is Valid`
              (if (`/Game/Boss/Character/BP_Boss.SendGroggyState` _bossactor)
                (bind (_location _rotator) (`/Game/Boss/Character/BP_Boss.PullTargetFrontOfBoss` (`self.BossActor`)))
                (`self.K2_SetActorLocationAndRotation` _location _rotator true)
                (`|PlayMontage` (`self.Mesh`) "/Game/Player/Animations/CriticalAttackAnimMontage.CriticalAttackAnimMontage")
                (else
                  (if (`self.Moving?`)
                    (`self.K2_SetActorRotation` (`self.CameraBasedMovementRotation`)))
                  (`|PlayMontage` (`self.Mesh`) "/Game/Player/Animations/LightAttack0_AnimMontage.LightAttack0_AnimMontage"))))))))))

(event `InputAxis|MoveRight/Left`
  (params (AxisValue :type "Float (single-precision)"))
  (bind _yaw (.yaw (`self.GetControlRotation`)))
  ; Character Movement
  (set `self.Moving?` true)
  (bind _returnvalue (`KismetMathLibrary.MakeVector` (stale `InputAxis|MoveForward/Backward` AxisValue) AxisValue))
  (if (== _returnvalue (0.0 0.0 0.0))
    (set `self.Moving?` false))
  (if (`self.LockedOn?`)
    (bind _returnvalue_2 (`KismetMathLibrary.MakeRotator` 0.0 0.0 (+ (.yaw (`KismetMathLibrary.MakeRotFromX` _returnvalue)) _yaw)))
    (set `self.InputBasedMovementRotation` _returnvalue_2)
    (else
      (set `self.CameraBasedMovementRotation` _returnvalue_2)))
  (if (`self.CanAct?`)
    (`self.AddMovementInput` (`KismetMathLibrary.GetRightVector` (`KismetMathLibrary.MakeRotator` 0.0 0.0 _yaw)) AxisValue)
    ;; camera following player (only when running left or right)
    (`self.AddControllerYawInput` (* AxisValue 0.21))))

(event `InputAction|StrongAttack(LeftHand)`
  (params (Key :type "Key Structure"))
  ; Strong Attack (Left Hand, Parry)
  (:`Pressed`
    (if (`self.CanAct?`)
      (if (`self.LockedOn?`)
        (`self.K2_SetActorRotation` (`self.CameraBasedMovementRotation`)))
      (`|PlayMontage` (`self.Mesh`) "/Game/Player/Animations/Parry_AnimMontage.Parry_AnimMontage"))))

(event `InputAxis|LookUp/Down`
  (params (AxisValue :type "Float (single-precision)"))
  ; Camera Movement
  ;; Look Up (Pitch)
  (if (not (`self.LockedOn?`))
    (set `SpringArmComponent.CameraRotationLagSpeed` 0.0 (`self.SpringArmComp`))
    (`self.AddControllerPitchInput` AxisValue)
    (if (== (+ (`self.GetInputAxisValue`) (`self.GetInputAxisValue`)) 0.0)
      (set `SpringArmComponent.CameraRotationLagSpeed` 4.0 (`self.SpringArmComp`)))))

(event `InputAxis|TurnRight/Left`
  (params (AxisValue :type "Float (single-precision)"))
  ; Camera Movement
  ;; Turn (Yaw)
  (if (not (`self.LockedOn?`))
    (set `SpringArmComponent.CameraRotationLagSpeed` 0.0 (`self.SpringArmComp`))
    (`self.AddControllerYawInput` AxisValue)
    (if (== (+ (`self.GetInputAxisValue`) (`self.GetInputAxisValue`)) 0.0)
      (set `SpringArmComponent.CameraRotationLagSpeed` 4.0 (`self.SpringArmComp`)))))

(event `InputAction|Attack(LeftHand)`
  (params (Key :type "Key Structure"))
  ; Light Attack (left Hand, Block)
  (:`Pressed`
    (if (`self.CanAct?`)
      (`self.K2_SetActorRotation` (`self.CameraBasedMovementRotation`))
      (`|PlayMontage` (`self.Mesh`) "/Game/Player/Animations/Block_AnimMontage.Block_AnimMontage")))
  (:`Released`
    (`self.StopAnimMontage` "/Game/Player/Animations/Block_AnimMontage.Block_AnimMontage")))

(fn `PlayerDamaged`
  (params (DamageValue :type "Float (double-precision)"))
  (if (`self.Invincible?`)
    _
    (elif (> DamageValue 0.0)
      (if (`self.Blocking?`)
        (`self.PlayAnimMontage` "/Game/Player/Animations/Blocked_AnimMontage.Blocked_AnimMontage")
        (set `self.PlayerHP` (- (`self.PlayerHP`) (* (`local.DamageValue`) 0.5)))
        (else
          (`self.PlayAnimMontage` "/Game/Player/Animations/Flinch_AnimMontage.Flinch_AnimMontage")
          (set `self.PlayerHP` (- (`self.PlayerHP`) (`local.DamageValue`))))))))

(fn `UserConstructionScript`)