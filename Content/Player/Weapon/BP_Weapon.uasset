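; BP_Weapon is the player's weapon, damaging BP_Boss when its WeaponCapsule begins overlapping it.
; The hit calls EnemyDamaged if the player character is in critical attack state 1 or is attacking, with the same damage either way.
; An Overlapping flag gates the event; it is set before the boss cast, so any overlap latches it, and this graph never clears it.
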(event `self.WeaponCapsule.OnComponentBeginOverlap`
  (params (OverlappedComponent :type "PrimitiveComponent Object Reference") (OtherActor :type "Actor Object Reference") (OtherComp :type "PrimitiveComponent Object Reference") (OtherBodyIndex :type Integer) (bFromSweep :type Boolean) (SweepResult :type "HitResult Structure (by ref)"))
  (if (not (`self.Overlapping?`))
    (set `self.Overlapping?` true)
    (bind _asbp_boss (cast `/Game/Boss/Character/BP_Boss` OtherActor))
    (bind _asbp_player_character (cast `/Game/Player/BP_PlayerCharacter` (`GameplayStatics.GetPlayerPawn` 0)))
    (if (== (`/Game/Player/BP_PlayerCharacter.CriticalAttackState` _asbp_player_character) 1)
      (`/Game/Boss/Character/BP_Boss.EnemyDamaged` _asbp_boss 50.0)
      (elif (`/Game/Player/BP_PlayerCharacter.Attacking?` _asbp_player_character)
        (`KismetSystemLibrary.PrintString` "50")
        (`/Game/Boss/Character/BP_Boss.EnemyDamaged` _asbp_boss 50.0)))))

(fn `UserConstructionScript`)