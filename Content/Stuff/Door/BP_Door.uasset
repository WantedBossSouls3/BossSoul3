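; Souls-style boss fog door that teleports the player to a set location and activates the boss on interaction.
; Box overlap registers the door on the player character and stores that player, clearing both on exit.
; Tick finds BP_Boss when its reference is invalid and re-shows the fog tip, via the game mode's HUD, while a player overlaps.
; Interact moves the stored player to TeleportLoc and calls the boss's ActivateMessage.
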(event `self.ReceiveTick`
  (params (DeltaSeconds :type "Float (single-precision)"))
  (`|ExecutionSequence`
    (:`then_0`
      (`/Engine/EditorBlueprintResources/StandardMacros.IsValid` (`self.Boss`)
        (:`Is Not Valid`
          (bind _returnvalue (`GameplayStatics.GetActorOfClass` "/Game/Boss/Character/BP_Boss.BP_Boss_C"))
          (set `self.Boss` _returnvalue))))
    (:`then_1`
      (`/Engine/EditorBlueprintResources/StandardMacros.IsValid` (`self.OverlappedPlayer`)
        (:`Is Valid`
          (bind _ingameui (`self.GetInGameUI`))
          (`/Game/UI/WBP_InGame.ChangeToFogTipText` _ingameui)
          (`/Game/UI/WBP_InGame.InteractionTipVisible` _ingameui))))))

(event `self.Box.OnComponentBeginOverlap`
  (params (OverlappedComponent :type "PrimitiveComponent Object Reference") (OtherActor :type "Actor Object Reference") (OtherComp :type "PrimitiveComponent Object Reference") (OtherBodyIndex :type Integer) (bFromSweep :type Boolean) (SweepResult :type "HitResult Structure (by ref)"))
  (bind _asbp_player_character (cast `/Game/Player/BP_PlayerCharacter` OtherActor))
  (set `/Game/Player/BP_PlayerCharacter.Door` self _asbp_player_character)
  (set `self.OverlappedPlayer` _asbp_player_character)
  (bind _asbp_soul_game_mode_level_and_state (cast `/Game/Blueprints/BP_SoulGameMode_LevelAndState` (`GameplayStatics.GetGameMode`))))

(event `self.Box.OnComponentEndOverlap`
  (params (OverlappedComponent :type "PrimitiveComponent Object Reference") (OtherActor :type "Actor Object Reference") (OtherComp :type "PrimitiveComponent Object Reference") (OtherBodyIndex :type Integer))
  (bind _asbp_player_character (cast `/Game/Player/BP_PlayerCharacter` OtherActor))
  (set `/Game/Player/BP_PlayerCharacter.Door` null _asbp_player_character)
  (bind _ingameui (`self.GetInGameUI`))
  (`/Game/UI/WBP_InGame.InteractionTipInvisible` _ingameui)
  (set `self.OverlappedPlayer` null))

(event `/Game/Utility/BPI_Stuff.Interact`
  (bind _overlappedplayer (`self.OverlappedPlayer`))
  (`/Engine/EditorBlueprintResources/StandardMacros.IsValid` _overlappedplayer
    (:`Is Valid`
      (`self.K2_SetActorLocation` _overlappedplayer (`self.Teleport Loc`) false true)
      (message `/Game/Utility/BPI_OnOff.Activate` (`self.Boss`)))))

(fn `UserConstructionScript`)