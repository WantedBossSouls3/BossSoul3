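; BP_Bonfire is a bonfire actor that detects when the player can rest at it and shows the interaction tip.
; Each Tick it asks BP_PlayerCharacter whether the player is looking at the bonfire and is within a fixed distance.
; The result sets RestingAvailable and shows or hides the bonfire tip on InGameUI.
; The UI reference is fetched lazily from the BP_InGame actor, a lookup marked as a placeholder.
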(event `self.ReceiveTick`
  (params (DeltaSeconds :type "Float (single-precision)"))
  (bind _ingameui (`self.InGameUI`))
  (bind _returnvalue (`ActorComponent.GetOwner` (`self.Bonfire`)))
  (`/Engine/EditorBlueprintResources/StandardMacros.IsValid` (`self.InGameUI`)
    (:`Is Valid`
      _)
    (:`Is Not Valid`
      ; 더미 바꿔야함
      (bind _returnvalue_2 (`GameplayStatics.GetActorOfClass` "/Game/UI/BP_InGame.BP_InGame_C"))
      (set `self.InGameUI` (`/Game/UI/BP_InGame.InGameUI` _returnvalue_2))))
  (bind _asbp_player_character (cast `/Game/Player/BP_PlayerCharacter` (`GameplayStatics.GetPlayerPawn` 0)))
  (bind _looking_ (`/Game/Player/BP_PlayerCharacter.IsPlayerLooking` _asbp_player_character _returnvalue))
  (if _looking_
    (if (< (`/Game/Player/BP_PlayerCharacter.DistanceBetweenPlayer` _asbp_player_character _returnvalue) 270.0)
      (`/Game/UI/WBP_InGame.ChangeToBonfireTipText` _ingameui)
      (`/Game/UI/WBP_InGame.InteractionTipVisible` _ingameui)
      (set `self.RestingAvailable?` true)
      (else
        (`/Game/UI/WBP_InGame.InteractionTipInvisible` (`self.InGameUI`))
        (set `self.RestingAvailable?` false)))
    (else
      (`/Game/UI/WBP_InGame.InteractionTipInvisible` (`self.InGameUI`))
      (set `self.RestingAvailable?` false))))

(fn `UserConstructionScript`)